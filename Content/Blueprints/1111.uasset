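; An actor that plays a flipbook-style mesh animation, swapping its static mesh through MeshArray while drifting along X.
; BeginPlay shows the first mesh and advances the index.
; Tick nudges the mesh component by a fixed per-frame transform, independent of delta time.
; A Delay in Tick, using FrameRate as seconds, throttles the swap to the next mesh, and the index wraps to loop.
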(event `self.ReceiveBeginPlay`
  (`StaticMeshComponent.SetStaticMesh` (`self.StaticMesh`) (`|GetArrayItem` (`self.MeshArray`)))
  (set `self.index` (+ (`self.index`) 1)))

(event `self.ReceiveTick`
  (params (DeltaSeconds :type "Float (single-precision)"))
  (`SceneComponent.K2_AddWorldTransform` (`self.StaticMesh`) (`KismetMathLibrary.MakeTransform` (0.01 0.0 0.0)) false false)
  (`KismetSystemLibrary.Delay` (`self.FrameRate`))
  (`StaticMeshComponent.SetStaticMesh` (`self.StaticMesh`) (`|GetArrayItem` (`self.MeshArray`) (`self.index`)))
  (set `self.index` (+ (`self.index`) 1))
  (if (>= (`self.index`) (`KismetArrayLibrary.Array_Length` (`self.MeshArray`)))
    (set `self.index` 0)))

(fn `UserConstructionScript`)