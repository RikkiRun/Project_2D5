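; BP_NPC_Bob is an NPC actor that plays a walking animation while drifting steadily along world Y.
; The animation is a mesh flipbook: a Delay on Tick, set by FrameRate, paces swaps of the StaticMesh through BobWalkingAnimArray in a loop.
; Movement is a fixed offset every Tick, so its speed depends on the game's frame rate.
; BeginPlay shows the first mesh and stores its world scale in PlayerScale.
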(event `self.ReceiveBeginPlay`
  (`StaticMeshComponent.SetStaticMesh` (`self.StaticMesh`) (`|GetArrayItem` (`self.BobWalkingAnimArray`)))
  (set `self.index` (+ (`self.index`) 1))
  (set `self.PlayerScale` (`SceneComponent.K2_GetComponentScale` (`self.StaticMesh`))))

(event `self.ReceiveTick`
  (params (DeltaSeconds :type "Float (single-precision)"))
  ;[1 1 1] AnimationHoldingwalking
  (`|ExecutionSequence`
    (:`then_0`
      (`KismetSystemLibrary.Delay` (`self.FrameRate`))
      (`StaticMeshComponent.SetStaticMesh` (`self.StaticMesh`) (`|GetArrayItem` (`self.BobWalkingAnimArray`) (`self.index`)))
      (set `self.index` (+ (`self.index`) 1))
      (if (>= (`self.index`) (`KismetArrayLibrary.Array_Length` (`self.BobWalkingAnimArray`)))
        (set `self.index` 0)))
    (:`then_1`
      (`self.K2_AddActorWorldTransform` (`KismetMathLibrary.MakeTransform` (0.0 0.3 0.0))))))

(fn `UserConstructionScript`)