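; Character actor that animates by flipbook-style swapping of static meshes from arrays for hold-walking, pickup, walking and throwing.
; Tick polls keys G, H, T and Y in priority order, using a Delay to pace frames through one shared Index that wraps per array.
; Both walking states also nudge the actor along world Y every tick.
; A separate MoveForward1 axis adds movement input from control rotation.
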(event `self.ReceiveBeginPlay`
  (`StaticMeshComponent.SetStaticMesh` (`self.StaticMesh`) (`|GetArrayItem` (`self.Hold&&WalkAnimArray`)))
  (set `self.index` (+ (`self.index`) 1))
  (set `self.PlayerScale` (`SceneComponent.K2_GetComponentScale` (`self.StaticMesh`))))

(event `self.ReceiveTick`
  (params (DeltaSeconds :type "Float (single-precision)"))
  (bind _output_get (set `self.IsHoldingwalking` (`PlayerController.IsInputKeyDown` (`GameplayStatics.GetPlayerController` 0) "G")))
  (if _output_get
    ;[1 1 1] AnimationHoldingwalking
    (`|ExecutionSequence`
      (:`then_0`
        (`KismetSystemLibrary.Delay` (`self.FrameRate`))
        (`StaticMeshComponent.SetStaticMesh` (`self.StaticMesh`) (`|GetArrayItem` (`self.Hold&&WalkAnimArray`) (`self.index`)))
        (set `self.index` (+ (`self.index`) 1))
        (if (>= (`self.index`) (`KismetArrayLibrary.Array_Length` (`self.Hold&&WalkAnimArray`)))
          (set `self.index` 0)))
      (:`then_1`
        (`self.K2_AddActorWorldTransform` (`KismetMathLibrary.MakeTransform` (0.0 1.0 0.0)))))
    (else
      (bind _output_get_2 (set `self.IsPickingup` (`PlayerController.IsInputKeyDown` (`GameplayStatics.GetPlayerController` 0) "H")))
      (if _output_get_2
        ;[1 1 1] AnimationPickup
        (`KismetSystemLibrary.Delay` (`self.FrameRate`))
        (`StaticMeshComponent.SetStaticMesh` (`self.StaticMesh`) (`|GetArrayItem` (`self.PickingupArray`) (`self.index`)))
        (set `self.index` (+ (`self.index`) 1))
        (if (>= (`self.index`) (`KismetArrayLibrary.Array_Length` (`self.PickingupArray`)))
          (set `self.index` 0))
        (else
          (bind _output_get_3 (set `self.IsWalking` (`PlayerController.IsInputKeyDown` (`GameplayStatics.GetPlayerController` 0) "T")))
          (if _output_get_3
            ;[1 1 1] AnimationWalking
            (`|ExecutionSequence`
              (:`then_0`
                (`KismetSystemLibrary.Delay` (`self.FrameRate`))
                (`StaticMeshComponent.SetStaticMesh` (`self.StaticMesh`) (`|GetArrayItem` (`self.WalkingArray`) (`self.index`)))
                (set `self.index` (+ (`self.index`) 1))
                (if (>= (`self.index`) (`KismetArrayLibrary.Array_Length` (`self.WalkingArray`)))
                  (set `self.index` 0)))
              (:`then_1`
                (`self.K2_AddActorWorldTransform` (`KismetMathLibrary.MakeTransform` (0.0 1.0 0.0)))))
            (elif (`PlayerController.IsInputKeyDown` (`GameplayStatics.GetPlayerController` 0) "Y")
              ;[1 1 1] AnimationThrowing
              (`KismetSystemLibrary.Delay` (`self.FrameRate`))
              (`StaticMeshComponent.SetStaticMesh` (`self.StaticMesh`) (`|GetArrayItem` (`self.ThrowingArray`) (`self.index`)))
              (set `self.index` (+ (`self.index`) 1))
              (if (>= (`self.index`) (`KismetArrayLibrary.Array_Length` (`self.ThrowingArray`)))
                (set `self.index` 0)))))))))

(event `InputAxis|MoveForward1`
  (params (AxisValue :type "Float (single-precision)"))
  (`self.AddMovementInput` (`KismetMathLibrary.GetForwardVector` (`KismetMathLibrary.MakeRotator` (.pitch (`self.GetControlRotation`)))) AxisValue))

(fn `UserConstructionScript`)