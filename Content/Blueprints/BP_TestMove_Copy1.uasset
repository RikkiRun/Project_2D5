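; Test movable pawn that animates its StaticMesh component as a flipbook by looping through an array of meshes.
; BeginPlay shows the first mesh, and Tick uses a Delay of FrameRate to throttle each swap and wrap the index.
; The MoveForward1 axis adds movement along the forward vector of a roll-only rotator built from control pitch, which always resolves to world X.
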(event `self.ReceiveBeginPlay`
  (`StaticMeshComponent.SetStaticMesh` (`self.StaticMesh`) (`|GetArrayItem` (`self.MeshArray`)))
  (set `self.index` (+ (`self.index`) 1))
  (set `self.PlayerScale` (`SceneComponent.K2_GetComponentScale` (`self.StaticMesh`))))

(event `self.ReceiveTick`
  (params (DeltaSeconds :type "Float (single-precision)"))
  (`KismetSystemLibrary.Delay` (`self.FrameRate`))
  (`StaticMeshComponent.SetStaticMesh` (`self.StaticMesh`) (`|GetArrayItem` (`self.MeshArray`) (`self.index`)))
  (set `self.index` (+ (`self.index`) 1))
  (if (>= (`self.index`) (`KismetArrayLibrary.Array_Length` (`self.MeshArray`)))
    (set `self.index` 0)))

(event `InputAxis|MoveForward1`
  (params (AxisValue :type "Float (single-precision)"))
  (`self.AddMovementInput` (`KismetMathLibrary.GetForwardVector` (`KismetMathLibrary.MakeRotator` (.pitch (`self.GetControlRotation`)))) AxisValue))

(fn `UserConstructionScript`)